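; BP_Weapon is a weapon with automatic fire that shoots BP_Bullet actors from its mesh's Muzzle socket.
; The duplicate Firing event and Fire function start a looping SpawnProjectile timer, clearing it only when both fire and release flags are true.
; Each shot adds smoke and sound.
; TraceFX spawns a Niagara trace toward a zero vector but is uncalled here, and the pickup-style sphere overlap only checks for the player character.
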(event OnComponentBeginOverlap(SkeletalMesh)
  (params (OverlappedComponent :type Primitive%20Component%20Object%20Reference) (OtherActor :type Actor%20Object%20Reference) (OtherComp :type Primitive%20Component%20Object%20Reference) (OtherBodyIndex :type Integer) (bFromSweep :type Boolean) (SweepResult :type Hit%20Result%20Structure%20%28by%20ref%29)))

(event OnComponentHit(SkeletalMesh)
  (params (HitComponent :type Primitive%20Component%20Object%20Reference) (OtherActor :type Actor%20Object%20Reference) (OtherComp :type Primitive%20Component%20Object%20Reference) (NormalImpulse :type Vector :default "0, 0, 0") (Hit :type Hit%20Result%20Structure%20%28by%20ref%29)))

(event OnComponentBeginOverlap(Sphere)
  (params (OverlappedComponent :type Primitive%20Component%20Object%20Reference) (OtherActor :type Actor%20Object%20Reference) (OtherComp :type Primitive%20Component%20Object%20Reference) (OtherBodyIndex :type Integer) (bFromSweep :type Boolean) (SweepResult :type Hit%20Result%20Structure%20%28by%20ref%29))
  (bind _asbp_third_person_character (Utilities|Casting|CastToBP_ThirdPersonCharacter OtherActor))
  (Utilities|IsValid _asbp_third_person_character))

(event Custom|Firing
  (params (Toggle :type Boolean) (Release :type Boolean))
  (bind _output_get (Variables|Condition|SetCanFire Toggle))
  (if _output_get
    (bind _returnvalue (Utilities|Time|SetTimerbyFunctionName 0 "SpawnProjectile" 0.1 true))
    (if Release
      (Utilities|Time|ClearandInvalidateTimerbyHandle _returnvalue))))

(event EventBeginPlay)

(event Collision|EventActorBeginOverlap
  (params (OtherActor :type Actor%20Object%20Reference)))

(event EventTick
  (params (DeltaSeconds :type Float%20%28single-precision%29)))

(fn ConstructionScript)

(fn SpawnProjectile
  (bind _skeletalmesh (Variables|Default|GetSkeletalMesh))
  (bind _returnvalue (Transformation|GetSocketTransform _skeletalmesh "Muzzle" "RTS_World"))
  (Game|SpawnActorfromClass "/Game/MyProject/Blueprints/Weapon/BP_Bullet.BP_Bullet_C" _returnvalue "AdjustIfPossibleButDontSpawnIfColliding" 0 0)
  (Effects|SpawnEmitterAttached "/Game/MyProject/Assets/Realistic_Starter_VFX_Pack_Vol2/Particles/Smoke/P_Smoke_A.P_Smoke_A" (Variables|Default|GetSkeletalMesh) "Muzzle")
  (Audio|PlaySoundatLocation "/Game/MyProject/Assets/StarterContent/Audio/Explosion01.Explosion01" (.Location (Math|Transform|BreakTransform _returnvalue)) "0, 0, 0" 0.1 0.1 0.0 0 0 0 0))

(fn TraceFX
  (bind _returnvalue (Niagara|SpawnSystematLocation (Variables|Default|GetTraceFXSystem) (Transformation|GetSocketLocation (Variables|Default|GetSkeletalMesh) "Muzzle")))
  (Niagara|SetNiagaraVariable(Vector3) _returnvalue "TraceTarget" "0, 0, 0"))

(fn Fire
  (params (Canfire :type Boolean) (Relese :type Boolean))
  (bind _output_get (Variables|Condition|SetCanFire Canfire))
  (if _output_get
    (bind _returnvalue (Utilities|Time|SetTimerbyFunctionName 0 "SpawnProjectile" 0.1 true))
    (if Relese
      (Utilities|Time|ClearandInvalidateTimerbyHandle _returnvalue))))