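; Generic character component that tracks one numeric parameter, identified by a gameplay tag, between minimum and maximum values.
; Increase and Decrease functions apply changes through a shared setter, which broadcasts the current value, maximum and tag.
; Reaching the maximum or dropping below the minimum clamps the value and also fires a Full or Empty notification.
; BeginPlay re-applies the starting value to broadcast the initial state.
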(event EventBeginPlay
  (Chages|SetCurrentParameter (Variables|Settings|GetCurrentValueParameter)))

(event EventTick
  (params (DeltaSeconds :type Float%20%28single-precision%29)))

(fn DecreaseParameter
  (params (Value :type Float%20%28double-precision%29))
  (bind _currentvalueparameter (Variables|Settings|GetCurrentValueParameter))
  (bind _returnvalue (- _currentvalueparameter Value))
  (bind _condition (Condition|HaveParameter _returnvalue))
  (if _condition
    (Chages|SetCurrentParameter _returnvalue)
    (else
      (Event|OnEmptyParameter))))

(fn IncreaseParameter
  (params (Value :type Float%20%28double-precision%29))
  (bind _currentvalueparameter (Variables|Settings|GetCurrentValueParameter))
  (bind _returnvalue (+ _currentvalueparameter Value))
  (if (>= _returnvalue (Variables|Settings|GetMaxValueParameter))
    (Event|OnFullParameter)
    (else
      (Chages|SetCurrentParameter _returnvalue))))

(fn SetCurrentParameter
  (params (v :type Float%20%28double-precision%29))
  (bind _output_get (Variables|Settings|SetCurrentValueParameter v))
  (Default|CallParameterChanged _output_get (Variables|Settings|GetMaxValueParameter) (Variables|Settings|GetGamerlay%20tag))
  (return))

(fn OnFullParameter
  (Chages|SetCurrentParameter (Variables|Settings|GetMaxValueParameter))
  (Default|CallParameterFull)
  (return))

(fn OnEmptyParameter
  (Chages|SetCurrentParameter (Variables|Settings|GetMinValueParameter))
  (Default|CallParameterEmpty)
  (return))

(fn HaveParameter
  (params (Value :type Float%20%28double-precision%29))
  (return (>= Value (Variables|Settings|GetMinValueParameter))))