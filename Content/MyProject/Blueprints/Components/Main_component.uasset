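; Main_component is a Blueprint component that holds one numeric parameter bounded by minimum and maximum values.
; DecreaseParameter and IncreaseParameter change the current value, handing off to IsEmptyParameter or IsFullParameter when a limit is reached, which clamps it to that bound.
; Despite their names, those two functions set the value rather than test it, and CurrentParameter serves as the getter.
; The event graph is unused.
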(event EventBeginPlay)

(event EventTick
  (params (DeltaSeconds :type Float%20%28single-precision%29)))

(fn DecreaseParameter
  (params (Value :type Float%20%28double-precision%29))
  (if (<= (- (Variables|Default|GetCurrentValueParameter) Value) (Variables|Default|GetMinValueParameter))
    (CallFunction|IsEmptyParameter)
    (else
      (Variables|Default|SetCurrentValueParameter (- (Variables|Default|GetCurrentValueParameter) Value)))))

(fn IncreaseParameter
  (params (Value :type Float%20%28double-precision%29))
  (if (>= (+ Value (Variables|Default|GetCurrentValueParameter)) (Variables|Default|GetMaxValueParameter))
    (CallFunction|IsFullParameter)
    (else
      (Variables|Default|SetCurrentValueParameter (+ Value (Variables|Default|GetCurrentValueParameter))))))

(fn CurrentParameter
  (return (Variables|Default|GetCurrentValueParameter)))

(fn IsFullParameter
  (bind _output_get (Variables|Default|SetCurrentValueParameter (Variables|Default|GetMaxValueParameter)))
  (return _output_get))

(fn IsEmptyParameter
  (bind _output_get (Variables|Default|SetCurrentValueParameter (Variables|Default|GetMinValueParameter)))
  (return _output_get))